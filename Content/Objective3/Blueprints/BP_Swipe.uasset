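; BP_Swipe is a touch-controlled, possessable Blueprint that rotates its Scene component as the player drags a finger across the screen.
; A press stores the start position and rotation and opens a Gate, so Tick applies the scaled drag delta as yaw and clamped pitch until release.
; Ending a touch on its StaticMesh makes the player controller possess it, unless Floor is set.
; BeginPlay enables the mouse cursor and touch events.
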(event OnInputTouchEnd(StaticMesh)
  (params (FingerIndex :type ETouchIndex%20Enum :default "Touch1") (TouchedComponent :type Primitive%20Component%20Object%20Reference))
  (if (not (Variables|Default|GetFloor?))
    (Pawn|Possess (Game|GetPlayerController 0) self)))

(event EventBeginPlay
  (bind _returnvalue (Game|GetPlayerController 0))
  (Variables|/Script/Engine.PlayerController|SetbShowMouseCursor _returnvalue true)
  (Variables|/Script/Engine.PlayerController|SetbEnableTouchEvents _returnvalue true))

(event EventTick
  (params (DeltaSeconds :type Float%20%28single-precision%29))
  (bind _returnvalue (Game|GetPlayerController 0))
  (bind _touchstart (Variables|Default|GetTouchStart))
  (bind _rotstart (Variables|Default|GetRotStart))
  (bind (_roll _pitch _yaw) (Math|Rotator|BreakRotator _rotstart))
  (bind (_locationx _locationy) (Class|PlayerController|GetInputTouchState _returnvalue "Touch1"))
  (bind _returnvalue_2 (Math|Vector2D|MakeVector2D _locationx _locationy))
  (bind _returnvalue_3 (- _returnvalue_2 _touchstart))
  (bind _returnvalue_4 (/ _returnvalue_3 5.0))
  (bind (_x _y) (Math|Vector2D|BreakVector2D _returnvalue_4))
  (Utilities|FlowControl|Gate true
    (:Exit
      (Transformation|SetWorldRotation (Variables|Default|GetScene) (Math|Rotator|MakeRotator 0.0 (Math|Float|Clamp(Float) (+ (* _y -1.0) _pitch) -2e+01 2e+01) (+ _x _yaw)) false false))))

(event Input|TouchEvents|InputTouch
  (params (Location :type Vector) (FingerIndex :type ETouchIndex%20Enum))
  (bind _returnvalue (Game|GetPlayerController 0))
  (bind (_locationx _locationy) (Class|PlayerController|GetInputTouchState _returnvalue "Touch1"))
  (:Pressed
    (Variables|Default|SetTouchStart (Math|Conversions|ToVector2D(Vector) Location))
    (Variables|Default|SetRotStart (Transformation|GetWorldRotation (Variables|Default|GetScene)))
    (Utilities|FlowControl|Gate true) ; enters at Open
  )
  (:Released
    (Utilities|FlowControl|Gate true) ; enters at Close
  ))

(fn ConstructionScript)