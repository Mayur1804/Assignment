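; BP_LoadJSON is an actor that spawns a BP_ActorToSpawn at a transform read from JSON on BeginPlay.
; It decodes a hardcoded JSON string through the VaRest subsystem, then builds the location and rotation from its number fields with unit scale.
; Despite the name, no file is read, as a LoadFileToString node sits unconnected in the graph.
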(event EventBeginPlay
  (bind _returnvalue (Class|VaRestSubsystem|DecodeJsonObject (|VaRestSubsystem) "{\"x\":200.0, \"y\":30.0, \"z\":150.0, \"RotX\":23.0, \"RotY\":70.0, \"RotZ\":120.0}"))
  (Game|SpawnActorfromClass "/Game/Objective2/Blueprints/BP_ActorToSpawn.BP_ActorToSpawn_C" (Math|Transform|MakeTransform (Math|Vector|MakeVector (Class|VaRestJsonObject|GetNumberField _returnvalue "x") (Class|VaRestJsonObject|GetNumberField _returnvalue "y") (Class|VaRestJsonObject|GetNumberField _returnvalue "z")) (Math|Rotator|MakeRotator (Class|VaRestJsonObject|GetNumberField _returnvalue "RotX") (Class|VaRestJsonObject|GetNumberField _returnvalue "RotY") (Class|VaRestJsonObject|GetNumberField _returnvalue "RotZ"))) "Undefined" 0 0))

(fn ConstructionScript)